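; BP_Ball is a projectile that removes itself when it hits parts of a tunnel.
; The construction script sets the projectile movement's initial and max speed from ProjectSpeed.
; On sphere overlap with a BP_Tunnel, it checks the WallMesh, HP and Enemies components, then destroys itself after a brief delay.
; A trailing debug print requires that same tunnel actor to also cast to BP_Player.
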(event OnComponentBeginOverlap(Sphere_0)
  (params (OverlappedComponent :type Primitive%20Component%20Object%20Reference) (OtherActor :type Actor%20Object%20Reference) (OtherComp :type Primitive%20Component%20Object%20Reference) (OtherBodyIndex :type Integer) (bFromSweep :type Boolean) (SweepResult :type Hit%20Result%20Structure%20%28by%20ref%29))
  (bind _sphere_0 (Variables|Default|GetSphere_0))
  (bind _asbp_tunnel (Utilities|Casting|CastToBP_Tunnel OtherActor))
  (if (Math|Boolean|ORBoolean (Class|PrimitiveComponent|IsOverlappingComponent _sphere_0 (Variables|/Game/InfiniteMatrix/Blueprints/BP_Tunnel.BP_Tunnel_C|GetWallMesh _asbp_tunnel)) (Class|PrimitiveComponent|IsOverlappingComponent _sphere_0 (Variables|/Game/InfiniteMatrix/Blueprints/BP_Tunnel.BP_Tunnel_C|GetHP _asbp_tunnel)) (Class|PrimitiveComponent|IsOverlappingComponent _sphere_0 (Variables|/Game/InfiniteMatrix/Blueprints/BP_Tunnel.BP_Tunnel_C|GetEnemies _asbp_tunnel)))
    (Utilities|FlowControl|Delay 0.1)
    (Actor|DestroyActor)
    (bind _asbp_player (Utilities|Casting|CastToBP_Player OtherActor))
    (Development|PrintString (Utilities|GetDisplayName _asbp_player))))

(event EventBeginPlay)

(event Collision|EventActorBeginOverlap
  (params (OtherActor :type Actor%20Object%20Reference)))

(event EventTick
  (params (DeltaSeconds :type Float%20%28single-precision%29)))

(fn ConstructionScript
  (bind _projectilemovement (Variables|Default|GetProjectileMovement))
  (bind _projectspeed (Variables|Default|GetProjectSpeed))
  (Variables|/Script/Engine.ProjectileMovementComponent|SetInitialSpeed _projectilemovement _projectspeed)
  (Variables|/Script/Engine.ProjectileMovementComponent|SetMaxSpeed _projectilemovement _projectspeed))