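; HPSpawner is an actor that spawns HealthPack actors in a chain.
; On BeginPlay it spawns the first pack at a fixed location and stores it as NewestHP, handing each new pack a reference back to itself.
; SpawnHPAtSpawnPoint spawns the next pack at the HPSpawnPoint of the newest one, so each pack sets where its successor appears.
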(event EventBeginPlay
  (CallFunction|SpawnHP "100.000000,0.000000,0.000000"))

(event Collision|EventActorBeginOverlap
  (params (OtherActor :type Actor%20Object%20Reference)))

(event EventTick
  (params (DeltaSeconds :type Float%20%28single-precision%29)))

(fn ConstructionScript)

(fn SpawnHP
  (params (SpawnLocation :type Vector))
  (bind _returnvalue (Game|SpawnActorfromClass "/Game/InfiniteMatrix/UI/HealthPack.HealthPack_C" (Math|Transform|MakeTransform SpawnLocation "0, 0, 0" "1.000000,1.000000,1.000000") "Undefined" "MultiplyWithRoot" 0 0))
  (bind _output_get (Variables|Default|SetNewestHP _returnvalue))
  (Variables|/Game/InfiniteMatrix/UI/HealthPack.HealthPack_C|SetHPSpawner _output_get self))

(fn SpawnHPatSpawnPoint
  (CallFunction|SpawnHP (Transformation|GetWorldLocation (Variables|/Game/InfiniteMatrix/UI/HealthPack.HealthPack_C|GetHPSpawnPoint (Variables|Default|GetNewestHP)))))